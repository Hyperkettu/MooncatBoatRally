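; BP_Boat is a physics-driven, player-controlled boat pawn steered through Enhanced Input, with its mapping context added on BeginPlay.
; The move action's Y axis applies thrust at EngineLocation along the flattened actor right vector, while X applies turning torque to the mesh.
; The same event opposes velocity along the actor forward vector, perpendicular to thrust, as sideways water damping, so this drag runs only when the input event fires.
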(event Input|EnhancedActionEvents|EnhancedInputActionIA_BoatMove
  (params (ActionValue :type Vector%202D%20Structure) (ElapsedSeconds :type Float%20%28double-precision%29) (TriggeredSeconds :type Float%20%28double-precision%29) (InputAction :type Input%20Action%20Object%20Reference :default "/Game/Input/IA_BoatMove.IA_BoatMove"))
  (bind _returnvalue (Transformation|GetActorForwardVector))
  (bind _returnvalue_2 (Transformation|GetActorRightVector))
  (bind _staticmesh (Variables|Default|GetStaticMesh))
  ;[0.15 0.15 0.15 0.5] Boat movement
  (Utilities|FlowControl|Sequence
    (:then_0
      (if (!= 0.0 (.y ActionValue))
        (Variables|Default|SetForceDirection (Math|Vector|MakeVector (.x _returnvalue_2) (.y _returnvalue_2) 0.0))
        (Class|PrimitiveComponent|AddForceatLocation _staticmesh (* (Variables|Default|GetForceDirection) (* (Math|Conversions|ToVector2D(Vector) (.y ActionValue)) (Variables|Default|GetThruster))) (Transformation|GetWorldLocation (Variables|Default|GetEngineLocation)) "None")))
    (:then_1
      (if (!= (.x ActionValue) 0.0)
        (Class|PrimitiveComponent|AddTorqueinDegrees _staticmesh (Math|Conversions|ToVector(Float) (* (.x ActionValue) (Variables|Default|GetTurnForce))) "None" true)))
    (:then_2
      (Physics|AddForce _staticmesh (* (* (Math|Vector|DotProduct _returnvalue (Transformation|GetVelocity)) (Variables|Default|GetWaterDamping)) (Math|Vector|NegateVector _returnvalue)) "None" true))))

(event EventBeginPlay
  (bind _asplayer_controller (Utilities|Casting|CastToPlayerController (Pawn|GetController)))
  (Input|AddMappingContext (PlayerController|LocalPlayerSubsystems|GetEnhancedInputLocalPlayerSubsystem _asplayer_controller) "/Game/Input/IMC_BoatInputMappiongContext.IMC_BoatInputMappiongContext" 0 "(bIgnoreAllPressedKeysUntilRelease=True,bForceImmediately=False,bNotifyUserSettings=False)"))

(event Collision|EventActorBeginOverlap
  (params (OtherActor :type Actor%20Object%20Reference)))

(event EventTick
  (params (DeltaSeconds :type Float%20%28single-precision%29)))

(fn ConstructionScript)